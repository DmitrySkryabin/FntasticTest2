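; AI controller for a turtle that alternates between moving and pausing.
; On begin play it stores the second TargetPoint found as the Hole location, then starts a one-shot timer.
; The timer clears the Move flag, waits briefly, restores it and re-arms itself, forming an endless stop-and-go cycle.
; While ItsOver is set, Tick looks up the turtle tagged Turtle2 and marks it as stopped.
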(event Custom|StopMoving
  (Variables|Default|SetMove false)
  (Utilities|FlowControl|Delay 1.0)
  (Variables|Default|SetMove true)
  (Utilities|Time|SetTimerbyEvent (delegate Custom|StopMoving) 2.0))

(event EventBeginPlay
  (|CallParentFunction)
  (bind _outactors (Actor|GetAllActorsOfClass "/Script/Engine.TargetPoint"))
  (Variables|Default|SetHole (Transformation|GetActorLocation (Utilities|Array|Get(acopy) _outactors 1)))
  (Utilities|Time|SetTimerbyEvent (delegate Custom|StopMoving) 2.0))

(event EventTick
  (params (DeltaSeconds :type Float%20%28single-precision%29))
  (|CallParentFunction DeltaSeconds)
  (if (Variables|Default|GetItsOver)
    (bind _outactors (Actor|GetAllActorswithTag "Turtle2"))
    (bind _asbp_turtle (Utilities|Casting|CastToBP_Turtle (Utilities|Array|Get(acopy) _outactors)))
    (Variables|/Game/Blueprints/BP_Turtle.BP_Turtle_C|SetTurtleIsStop _asbp_turtle true)))

(fn ConstructionScript
  (|CallParentFunction))