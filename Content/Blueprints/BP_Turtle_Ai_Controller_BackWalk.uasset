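; AI controller for a back-walking turtle, periodically switching its destination between its start point and the target hole.
; BeginPlay takes both positions from level TargetPoints by array index.
; A self-rearming timer points Hole at the start for half a second, then back at the target, until ItsOver.
; Once ItsOver is set, Tick flags the turtle tagged "Turtle3" as stopped; movement itself is not implemented here.
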(event Custom|CustomEvent_0
  (Variables|Default|SetMove false)
  (Variables|Default|SetHole (Variables|Default|GetCreatePosition))
  (Variables|Default|SetMove true)
  (Utilities|FlowControl|Delay 0.5)
  (Variables|Default|SetHole (Variables|Default|GetTargetPosition))
  (if (Variables|Default|GetItsOver)
    (Variables|Default|SetMove false)
    (else
      (Utilities|Time|SetTimerbyEvent (delegate Custom|CustomEvent_0) 1.0))))

(event EventBeginPlay
  (|CallParentFunction)
  (bind _outactors (Actor|GetAllActorsOfClass "/Script/Engine.TargetPoint"))
  (Variables|Default|SetCreatePosition (Transformation|GetActorLocation (Utilities|Array|Get(acopy) _outactors 3)))
  (bind _outactors_2 (Actor|GetAllActorsOfClass "/Script/Engine.TargetPoint"))
  (bind _output_get (Variables|Default|SetHole (Transformation|GetActorLocation (Utilities|Array|Get(acopy) _outactors_2 2))))
  (Variables|Default|SetTargetPosition _output_get)
  (Utilities|Time|SetTimerbyEvent (delegate Custom|CustomEvent_0) 1.0))

(event EventTick
  (params (DeltaSeconds :type Float%20%28single-precision%29))
  (|CallParentFunction DeltaSeconds)
  (if (Variables|Default|GetItsOver)
    (bind _outactors (Actor|GetAllActorswithTag "Turtle3"))
    (bind _asbp_turtle (Utilities|Casting|CastToBP_Turtle (Utilities|Array|Get(acopy) _outactors)))
    (Variables|/Game/Blueprints/BP_Turtle.BP_Turtle_C|SetTurtleIsStop _asbp_turtle true)))

(fn ConstructionScript
  (|CallParentFunction))