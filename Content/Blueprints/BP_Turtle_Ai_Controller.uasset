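; AI controller that walks a turtle to a goal location, taken at BeginPlay from the first TargetPoint in the level.
; While Start is set, Tick calls Moving, which either moves toward that point or halts, depending on the Move flag.
; On arrival it sets ItsOver and plays a bell once if MusicPlay is set.
; Tick then flags the first actor tagged Turtle1, cast to BP_Turtle, as stopped.
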(event EventBeginPlay
  (bind _outactors (Actor|GetAllActorsOfClass "/Script/Engine.TargetPoint"))
  (Variables|Default|SetHole (Transformation|GetActorLocation (Utilities|Array|Get(acopy) _outactors))))

(event EventTick
  (params (DeltaSeconds :type Float%20%28single-precision%29))
  (if (Variables|Default|GetStart)
    (CallFunction|Moving)
    (if (Variables|Default|GetItsOver)
      (bind _outactors (Actor|GetAllActorswithTag "Turtle1"))
      (bind _asbp_turtle (Utilities|Casting|CastToBP_Turtle (Utilities|Array|Get(acopy) _outactors)))
      (Variables|/Game/Blueprints/BP_Turtle.BP_Turtle_C|SetTurtleIsStop _asbp_turtle true))))

(fn ConstructionScript)

(fn Moving
  (if (Variables|Default|GetMove)
    (bind _returnvalue (AI|Navigation|MovetoLocation (Variables|Default|GetHole) -1.0 true true false true 0))
    (switch Utilities|FlowControl|Switch|SwitchonEPathFollowingRequestResult _returnvalue
      (:AlreadyAtGoal
        (Variables|Default|SetItsOver true)
        (if (Variables|Default|GetMusicPlay)
          (Audio|PlaySound2D "/Game/Assets/Bell_Sound.Bell_Sound" 0.1 1.0 0.0 0 0)
          (Variables|Default|SetMusicPlay false))))
    (else
      (AI|Navigation|StopMovement))))